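; Rocket projectile that explodes when its movement component stops, with camera shake and controller rumble on spawn.
; On a blocking hit it plays explosion effects, triggers destruction on Chaos-tagged BP_ChaoesDestruct3 actors and expires shortly after.
; That hit also sends DamageMessage with the impact point to pawns found by a sphere overlap.
; Every stop hides the mesh and spawns an ExplosionImpulse actor at the impact point, even without a blocking hit.
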(event OnProjectileStop(ProjectileMovement)
  (params (ImpactResult :type Hit%20Result%20Structure%20%28by%20ref%29))
  (CallFunction|ProjectileStop ImpactResult))

(event Custom|Projectile%20Stop
  (params (Hit%20Result :type Hit%20Result%20Structure))
  (bind (_bblockinghit _binitialoverlap _time _distance _location _impactpoint _normal _impactnormal _physmat _hitactor) (Collision|BreakHitResult Hit%20Result))
  (Utilities|FlowControl|Sequence
    (:then_0
      (Development|SetHiddeninGame (Variables|Default|GetMesh) true false)
      (if _bblockinghit
        (Utilities|FlowControl|Sequence
          (:then_0
            (Effects|SpawnEmitteratLocation "/Game/MilitaryWeapSilver/FX/P_RocketLauncher_Explosion_01.P_RocketLauncher_Explosion_01" _impactpoint)
            (Audio|PlaySoundatLocation "/Game/MilitaryWeapSilver/Sound/RocketLauncher/Cues/RocketLauncher_Explosion_Cue.RocketLauncher_Explosion_Cue" _impactpoint "0, 0, 0" 1.0 1.0 0.0 0 0 0 0)
            (Physics|SetSimulatePhysics (Variables|Default|GetMesh) true)
            (if (Actor|ActorHasTag _hitactor "Chaos")
              (bind _asbp_chaoes_destruct_3 (Utilities|Casting|CastToBP_ChaoesDestruct3 _hitactor)
                (:then
                  (Default|Destrction _asbp_chaoes_destruct_3))
                (:CastFailed
                  _)))
            (Actor|SetLifeSpan 0.2))
          (:then_1
            (bind _outactors (Collision|SphereOverlapActors (Transformation|GetActorLocation) 6e+02 (Utilities|Array|MakeArray "ObjectTypeQuery3") 0))
            (for _array_element _outactors
              (Class|BPITakeDamage|Damage(Message) _array_element _impactpoint))))))
    (:then_1
      (Game|SpawnActorfromClass "/Game/Blueprint/ExplosionImpulse.ExplosionImpulse_C" (Math|Transform|MakeTransform _impactpoint "0, 0, 0" "1.000000,1.000000,1.000000") "AlwaysSpawn" "MultiplyWithRoot" 0 0))))

(event EventBeginPlay
  (Camera|PlayWorldCameraShake "/Game/Blueprint/BP_CameraShake2.BP_CameraShake2_C" (Transformation|GetActorLocation) 0.0 5e+02)
  (Game|Feedback|ClientPlayForceFeedback (Class|MyBlueprintFunctionLibrary|GetActivePlayerController) "/Game/_Game/Input/ForceFeedback/FF_RiflePickup.FF_RiflePickup" "None" false false false))

(event Collision|EventActorBeginOverlap
  (params (OtherActor :type Actor%20Object%20Reference)))

(event EventTick
  (params (DeltaSeconds :type Float%20%28single-precision%29)))

(fn ConstructionScript)