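; Moving laser actor that swings its ItemMesh2 component either left-right or up-down, depending on LaserMode.
; On BeginPlay it starts the timeline for that mode, which drives relative yaw for Left Right or roll for Up Down, scaled by RotateValue.
; Its widget starts hidden and is shown or hidden through the ShowHideUIinBP event.
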(event EventBeginPlay
  (Rendering|SetVisibility (Variables|Default|GetWidget) false false)
  (switch Utilities|FlowControl|Switch|SwitchonE_LaserMode (Variables|Default|GetLaserMode)
    (:NewEnumerator1
      (bind _newtrack_0 (Timeline|Rotate PlayFromStart)
        (:Update
          (Transformation|SetRelativeRotation (Variables|Default|GetItemMesh2) (Math|Rotator|MakeRotator 0.0 0.0 (* _newtrack_0 (Variables|Default|GetRotate%20Value))) false false))))
    (:NewEnumerator2
      (bind _newtrack_0_2 (Timeline|Timeline PlayFromStart)
        (:Update
          (Transformation|SetRelativeRotation (Variables|Default|GetItemMesh2) (Math|Rotator|MakeRotator (* _newtrack_0_2 (Variables|Default|GetRotate%20Value)) 0.0 0.0) false false))))))

(event EventTick
  (params (DeltaSeconds :type Float%20%28single-precision%29)))

(event EventShowHideUIinBP
  (params (Show :type Boolean))
  (Rendering|SetVisibility (Variables|Default|GetWidget) Show false))

(fn ConstructionScript)