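; A colour-locked door that the player opens by interacting while holding the required coloured keys.
; On BeginPlay it shows red, blue and green key labels according to KeysRequired, and overlapping players get an interact prompt.
; Activate checks the character's ColouredKeys against KeysRequired, stopping at the first missing colour.
; On success it clears all the character's keys and a Timeline swings the door open; either outcome shows a HUD message.
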(event Custom|break%20loop
  (Utilities|Array|ForEachLoopwithBreak (Variables|Default|GetkeysRequired)) ; enters at Break
)

(event EventBeginPlay
  (Utilities|FlowControl|Sequence
    (:then_0
      (Rendering|SetVisibility (Variables|Default|GetRedKeyText) (Utilities|Array|ContainsItem (Variables|Default|GetkeysRequired) "RED") false))
    (:then_1
      (Rendering|SetVisibility (Variables|Default|GetBlueKeyText) (Utilities|Array|ContainsItem (Variables|Default|GetkeysRequired) "BLUE") false))
    (:then_2
      (Rendering|SetVisibility (Variables|Default|GetGreenKeyText) (Utilities|Array|ContainsItem (Variables|Default|GetkeysRequired) "GREEN") false))))

(event Collision|EventActorBeginOverlap
  (params (OtherActor :type Actor%20Object%20Reference))
  (if (Utilities|DoesObjectImplementInterface OtherActor "/Game/Blueprint/Interfaces-Enums/BPI_Player.BPI_Player_C")
    (Class|BPIPlayer|InteractButtonUIDisplay(Message) OtherActor "Interact with E")))

(event EventTick
  (params (DeltaSeconds :type Float%20%28single-precision%29)))

(event EventActivate
  (params (Shooter%20Character%20Ref :type BP%20Shooter%20Character%20Object%20Reference))
  (Variables|Default|SetShooter%20Character%20Ref Shooter%20Character%20Ref)
  (for _array_element (Variables|/Script/A_Afridi_Shahid.ShooterCharacter|GetcolouredKeys Shooter%20Character%20Ref)
    (Utilities|Array|Add (Variables|Default|GettestArray) (Variables|/Script/A_Afridi_Shahid.ColouredKey|GetkeyColourEnum _array_element)))
  (bind _array_element_2 (Utilities|Array|ForEachLoopwithBreak (Variables|Default|GetkeysRequired))
    (:LoopBody
      (bind _output_get (Variables|Default|SetCondition (Utilities|Array|ContainsItem (Variables|Default|GettestArray) _array_element_2)))
      (if (not _output_get)
        (CallFunction|BreakLoop)))
    (:Completed
      (if (Variables|Default|GetCondition)
        (Default|ShowMessageInfoWIthAnim (Variables|/Game/_Game/Character/BP_ShooterCharacter.BP_ShooterCharacter_C|GetWBP_MainWidget%20ref Shooter%20Character%20Ref) "/Game/UI_Assert/T_U_Message_ContainerGreen.T_U_Message_ContainerGreen" "Success" "(R=1.000000,G=1.000000,B=1.000000,A=1.000000)")
        (Utilities|Array|Clear (Variables|/Script/A_Afridi_Shahid.ShooterCharacter|GetcolouredKeys (Variables|Default|GetShooter%20Character%20Ref)))
        (bind _dooropen (Timeline|Timeline PlayFromStart)
          (:Update
            (Transformation|SetRelativeRotation (Variables|Default|GetCube) (Math|Rotator|MakeRotator 0.0 0.0 _dooropen) false false)))
        (else
          (Default|ShowMessageInfoWIthAnim (Variables|/Game/_Game/Character/BP_ShooterCharacter.BP_ShooterCharacter_C|GetWBP_MainWidget%20ref Shooter%20Character%20Ref) "/Game/UI_Assert/T_U_Message_ContainerGreen.T_U_Message_ContainerGreen" "Collect all keys first" "(R=1.000000,G=1.000000,B=1.000000,A=1.000000)"))))))

(fn ConstructionScript)