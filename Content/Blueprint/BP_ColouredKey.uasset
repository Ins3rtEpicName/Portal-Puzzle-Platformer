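; BP_ColouredKey is a coloured key pickup that disappears when an actor overlaps it.
; After a short delay, any overlap hides the Sphere, deactivates the BoxComponent and disables collision on both, without destroying the actor.
; ShowColor maps KeyColourEnum to red, blue or green and applies it through a dynamic material instance's Color parameter.
; Nothing in this Blueprint calls ShowColor or records who collected the key.
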(event EventBeginPlay)

(event Collision|EventActorBeginOverlap
  (params (OtherActor :type Actor%20Object%20Reference))
  (bind _sphere (Variables|Default|GetSphere))
  (Utilities|FlowControl|Delay 0.2)
  (Rendering|SetVisibility _sphere false false)
  (Components|Activation|SetActive (Variables|Default|GetboxComponent) false false)
  (Collision|SetCollisionEnabled _sphere "NoCollision"))

(event EventTick
  (params (DeltaSeconds :type Float%20%28single-precision%29)))

(fn ConstructionScript)

(fn ShowColor
  (bind _sphere (Variables|Default|GetSphere))
  (switch Utilities|FlowControl|Switch|SwitchonKeyColour (Variables|Default|GetkeyColourEnum)
    (:RED
      (Variables|Default|SetkeyColour (Utilities|Struct|MakeLinearColor 1.0 0.0 0.0 1.0)))
    (:BLUE
      (Variables|Default|SetkeyColour (Utilities|Struct|MakeLinearColor 0.0 0.0 1.0 1.0)))
    (:GREEN
      (Variables|Default|SetkeyColour (Utilities|Struct|MakeLinearColor 0.0 1.0 0.0 1.0))))
  (bind _returnvalue (Rendering|Material|CreateDynamicMaterialInstance _sphere 0 (Rendering|Material|GetMaterial _sphere 0) "None" :!class /Script/Engine.PrimitiveComponent))
  (Rendering|Material|SetVectorParameterValue _returnvalue "Color" (Variables|Default|GetkeyColour) :!class /Script/Engine.MaterialInstanceDynamic))