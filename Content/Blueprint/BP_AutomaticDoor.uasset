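; BP_AutomaticDoor is a two-panel sliding door that opens when something enters its Box trigger and closes when it leaves.
; Begin overlap plays the Slide timeline, which lerps the left and right panels' relative locations from current to new positions; end overlap reverses it.
; Both overlap events play the same 2D sound and print a debug message, with no filtering of the overlapping actor.
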(event OnComponentBeginOverlap(Box)
  (params (OverlappedComponent :type Primitive%20Component%20Object%20Reference) (OtherActor :type Actor%20Object%20Reference) (OtherComp :type Primitive%20Component%20Object%20Reference) (OtherBodyIndex :type Integer) (bFromSweep :type Boolean) (SweepResult :type Hit%20Result%20Structure%20%28by%20ref%29))
  (Audio|PlaySound2D "/Engine/VREditor/Sounds/UI/Scaling_Up.Scaling_Up" 1.0 1.0 0.0 0 0)
  (Development|PrintString "Enter")
  (bind _slidingdoor (Timeline|Slide Play)
    (:Update
      (Transformation|SetRelativeLocation (Variables|Default|GetLeftSlidingDoor) (Math|Vector|Lerp(Vector) (Variables|Default|GetCurrentLeft) (Variables|Default|GetNewLeft) _slidingdoor) false false)
      (Transformation|SetRelativeLocation (Variables|Default|GetRightSlidingDoor) (Math|Vector|Lerp(Vector) (Variables|Default|GetCurrentRight) (Variables|Default|GetNewRight) _slidingdoor) false false))))

(event OnComponentEndOverlap(Box)
  (params (OverlappedComponent :type Primitive%20Component%20Object%20Reference) (OtherActor :type Actor%20Object%20Reference) (OtherComp :type Primitive%20Component%20Object%20Reference) (OtherBodyIndex :type Integer))
  (Audio|PlaySound2D "/Engine/VREditor/Sounds/UI/Scaling_Up.Scaling_Up" 1.0 1.0 0.0 0 0)
  (Development|PrintString "Exit")
  (bind _slidingdoor (Timeline|Slide Reverse)
    (:Update
      (Transformation|SetRelativeLocation (Variables|Default|GetLeftSlidingDoor) (Math|Vector|Lerp(Vector) (Variables|Default|GetCurrentLeft) (Variables|Default|GetNewLeft) _slidingdoor) false false)
      (Transformation|SetRelativeLocation (Variables|Default|GetRightSlidingDoor) (Math|Vector|Lerp(Vector) (Variables|Default|GetCurrentRight) (Variables|Default|GetNewRight) _slidingdoor) false false))))

(event EventBeginPlay)

(event Collision|EventActorBeginOverlap
  (params (OtherActor :type Actor%20Object%20Reference)))

(event EventTick
  (params (DeltaSeconds :type Float%20%28single-precision%29)))

(fn ConstructionScript)