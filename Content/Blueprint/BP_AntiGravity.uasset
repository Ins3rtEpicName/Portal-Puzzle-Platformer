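; BP_AntiGravity is an interactable zone that applies a configurable gravity value to the shooter character.
; Overlapping its box shows an enable or disable prompt on actors implementing BPI_Player, depending on whether GravityValue equals 1.
; Activate passes GravityValue to the character's AntiGravity function and shows a widget message, playing a montage when gravity is altered.
; The construction script labels a TextRender with the value, which is hidden at BeginPlay.
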(event OnComponentBeginOverlap(Box)
  (params (OverlappedComponent :type Primitive%20Component%20Object%20Reference) (OtherActor :type Actor%20Object%20Reference) (OtherComp :type Primitive%20Component%20Object%20Reference) (OtherBodyIndex :type Integer) (bFromSweep :type Boolean) (SweepResult :type Hit%20Result%20Structure%20%28by%20ref%29))
  (if (Utilities|DoesObjectImplementInterface OtherActor "/Game/Blueprint/Interfaces-Enums/BPI_Player.BPI_Player_C")
    (if (== (Variables|Default|GetGravity%20Value) 1.0)
      (Class|BPIPlayer|InteractButtonUIDisplay(Message) OtherActor "Diable-Gravity with E")
      (else
        (Class|BPIPlayer|InteractButtonUIDisplay(Message) OtherActor "Enable-Gravity with E")))))

(event EventBeginPlay
  (Rendering|SetVisibility (Variables|Default|GetTextRender) false false))

(event EventActivate
  (params (Shooter%20Character%20Ref :type BP%20Shooter%20Character%20Object%20Reference))
  (bind _wbp_mainwidget_ref (Variables|/Game/_Game/Character/BP_ShooterCharacter.BP_ShooterCharacter_C|GetWBP_MainWidget%20ref Shooter%20Character%20Ref))
  (bind _gravity_value (Variables|Default|GetGravity%20Value))
  (Default|Anti-Gravity Shooter%20Character%20Ref _gravity_value)
  (if (== _gravity_value 1.0)
    (Default|ShowMessageInfoWIthAnim _wbp_mainwidget_ref "/Game/UI_Assert/T_U_Message_ContainerPurple.T_U_Message_ContainerPurple" "Anti-Gravity is off" "(R=1.000000,G=1.000000,B=1.000000,A=1.000000)")
    (else
      (Default|ShowMessageInfoWIthAnim _wbp_mainwidget_ref "/Game/UI_Assert/T_U_Message_ContainerRed.T_U_Message_ContainerRed" "Anti-Gravity in Action" "(R=1.000000,G=1.000000,B=1.000000,A=1.000000)")
      (Default|PlayMontage Shooter%20Character%20Ref "/Game/Blueprint/Animations/Emotes/Cosmic_Rift1_Montage.Cosmic_Rift1_Montage" 1.5))))

(fn ConstructionScript
  (Rendering|Components|TextRender|SetText (Variables|Default|GetTextRender) (Utilities|Text|ToText(String) (Utilities|String|Append "Gravity Force : " (Utilities|String|ToString(Float) (Variables|Default|GetGravity%20Value))))))