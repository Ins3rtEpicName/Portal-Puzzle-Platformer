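; BP_WindBlower is a switchable fan that launches players who enter its trigger box while it runs.
; Activate plays a sound and ramps rotation with a timeline, whose updates also set a looping timer for continuous spin.
; Deactivate stops the sound and reverses the timeline, pausing that timer as the blades slow.
; Box overlap uses BPI_Player to display a message and launch the player with Force and HowLong.
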(event OnComponentBeginOverlap(Box)
  (params (OverlappedComponent :type Primitive%20Component%20Object%20Reference) (OtherActor :type Actor%20Object%20Reference) (OtherComp :type Primitive%20Component%20Object%20Reference) (OtherBodyIndex :type Integer) (bFromSweep :type Boolean) (SweepResult :type Hit%20Result%20Structure%20%28by%20ref%29))
  (if (Variables|Default|GetIs%20Fan%20On)
    (if (Utilities|DoesObjectImplementInterface OtherActor "/Game/Blueprint/Interfaces-Enums/BPI_Player.BPI_Player_C")
      (Class|BPIPlayer|InteractButtonUIDisplay(Message) OtherActor "SIIIUUU!")
      (bind _player_ref (Class|BPIPlayer|GetPlayerRef(Message) OtherActor))
      (Default|LaunchPlayer _player_ref (Variables|Default|GetForce) (Variables|Default|GetHow%20long)))))

(event Custom|Activate
  (Variables|Default|SetIs%20Fan%20On true)
  (bind _returnvalue (Audio|SpawnSound2D "/Game/UI_Assert/fan_on_sound_Cue.fan_on_sound_Cue" 0.5 1.0 0.0 0))
  (bind _newtrack_0 (Timeline|FanTimeline PlayFromStart)
    (:Update
      (Transformation|AddRelativeRotation (Variables|Default|GetFan) (Math|Rotator|MakeRotator 0.0 0.0 (Math|Float|Lerp 0.0 (Variables|Default|GetFan%20Speed) _newtrack_0)) false false)
      (if (not (Variables|Default|GetIs%20Fan%20On))
        (Utilities|Time|PauseTimerbyHandle (stale _returnvalue_2))
        (else
          (bind _returnvalue_2 (Utilities|Time|SetTimerbyEvent (delegate Custom|FanOn) (Utilities|Time|GetWorldDeltaSeconds) true)))))))

(event Custom|Deactivate
  (Variables|Default|SetIs%20Fan%20On false)
  (Audio|Components|Audio|Stop (stale Custom|Activate _returnvalue))
  (bind _newtrack_0 (Timeline|FanTimeline ReverseFromEnd)
    (:Update
      (Transformation|AddRelativeRotation (Variables|Default|GetFan) (Math|Rotator|MakeRotator 0.0 0.0 (Math|Float|Lerp 0.0 (Variables|Default|GetFan%20Speed) _newtrack_0)) false false)
      (if (not (Variables|Default|GetIs%20Fan%20On))
        (Utilities|Time|PauseTimerbyHandle (stale _returnvalue))
        (else
          (bind _returnvalue (Utilities|Time|SetTimerbyEvent (delegate Custom|FanOn) (Utilities|Time|GetWorldDeltaSeconds) true)))))))

(event Custom|FanOn
  (Transformation|AddRelativeRotation (Variables|Default|GetFan) (Math|Rotator|MakeRotator 0.0 0.0 (Variables|Default|GetFan%20Speed)) false false))

(fn ConstructionScript)