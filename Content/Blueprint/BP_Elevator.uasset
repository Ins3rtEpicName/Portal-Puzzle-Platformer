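; Interactive elevator that fakes a ride by teleporting itself and the player to a preset transform.
; A proximity box shows the interact prompt, and Activate slides both doors open with timelines.
; The inside trigger closes the doors, plays running audio, waits, teleports elevator and player, then reopens.
; The outside trigger closes the doors behind the exiting player and shows a new-mission message, with DoOnce keeping triggers single-use.
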(event OnComponentBeginOverlap(Box)
  (params (OverlappedComponent :type Primitive%20Component%20Object%20Reference) (OtherActor :type Actor%20Object%20Reference) (OtherComp :type Primitive%20Component%20Object%20Reference) (OtherBodyIndex :type Integer) (bFromSweep :type Boolean) (SweepResult :type Hit%20Result%20Structure%20%28by%20ref%29))
  (Utilities|FlowControl|DoOnce false
    (:Completed
      (if (Utilities|DoesObjectImplementInterface OtherActor "/Game/Blueprint/Interfaces-Enums/BPI_Player.BPI_Player_C")
        (Class|BPIPlayer|InteractButtonUIDisplay(Message) OtherActor "Interact with E")))))

(event OnComponentBeginOverlap(Insider)
  (params (OverlappedComponent :type Primitive%20Component%20Object%20Reference) (OtherActor :type Actor%20Object%20Reference) (OtherComp :type Primitive%20Component%20Object%20Reference) (OtherBodyIndex :type Integer) (bFromSweep :type Boolean) (SweepResult :type Hit%20Result%20Structure%20%28by%20ref%29))
  (bind _returnvalue (Transformation|GetActorLocation))
  (bind (_x _y _z) (Math|Vector|BreakVector _returnvalue))
  (if (Actor|ActorHasTag OtherActor "Player")
    (Utilities|FlowControl|DoOnce false
      (:Completed
        (Variables|Default|SetIs%20inside true)
        (Audio|PlaySound2D "/Game/UI_Assert/elevatro_inside_runnign_sound.elevatro_inside_runnign_sound" 1.0 1.0 0.0 0 0)
        (bind _newtrack_0 (Timeline|Timeline_0 Play)
          (:Update
            (Transformation|SetRelativeLocation (Variables|Default|GetDoor1) (Math|Vector|MakeVector (Math|Float|Lerp -177.939266 -57.889229 _newtrack_0) 202.361636 129.0) false false)
            (Transformation|SetRelativeLocation (Variables|Default|GetDoor2) (Math|Vector|MakeVector (Math|Float|Lerp 174.0 59.0 _newtrack_0) 202.361636 129.0) false false))
          (:Finished
            (Utilities|FlowControl|Delay 3.7)
            (Transformation|SetActorTransform (Variables|Default|GetElevator%20Teleport%20Transform) false true)
            (Utilities|FlowControl|Delay 0.2)
            (Transformation|SetActorLocation OtherActor (Math|Vector|MakeVector _x _y (+ _z 2e+01)) false false)
            (Transformation|SetActorRotation OtherActor (Transformation|GetActorRotation))
            (CallFunction|Re-open)
            (Audio|PlaySound2D "/Game/UI_Assert/elevator_open_sound.elevator_open_sound" 1.0 1.0 0.0 0 0)))))))

(event OnComponentBeginOverlap(Outsider)
  (params (OverlappedComponent :type Primitive%20Component%20Object%20Reference) (OtherActor :type Actor%20Object%20Reference) (OtherComp :type Primitive%20Component%20Object%20Reference) (OtherBodyIndex :type Integer) (bFromSweep :type Boolean) (SweepResult :type Hit%20Result%20Structure%20%28by%20ref%29))
  (if (Variables|Default|GetIs%20inside)
    (if (Actor|ActorHasTag OtherActor "Player")
      (Utilities|FlowControl|DoOnce false
        (:Completed
          (Variables|Default|SetIs%20inside false)
          (Class|BPIPlayer|InteractButtonUIDisplay(Message) OtherActor "New Mission. Good Luck")
          (bind _newtrack_0 (Timeline|Timeline_1 PlayFromStart)
            (:Update
              (Transformation|SetRelativeLocation (Variables|Default|GetDoor1) (Math|Vector|MakeVector (Math|Float|Lerp -177.939266 -57.889229 _newtrack_0) 202.361636 129.0) false false)
              (Transformation|SetRelativeLocation (Variables|Default|GetDoor2) (Math|Vector|MakeVector (Math|Float|Lerp 174.0 59.0 _newtrack_0) 202.361636 129.0) false false))))))))

(event Custom|Re-open
  (Utilities|FlowControl|Sequence
    (:then_0
      (Utilities|FlowControl|DoOnce false) ; enters at Reset
    )
    (:then_1
      (Audio|PlaySound2D "/Engine/VREditor/Sounds/UI/Enter_Simulate.Enter_Simulate" 1.5 1.0 0.0 0 0)
      (Variables|Default|SetOpen%20Stste true)
      (bind _newtrack_0 (Timeline|Timeline PlayFromStart)
        (:Update
          (Transformation|SetRelativeLocation (Variables|Default|GetDoor1) (Math|Vector|MakeVector (Math|Float|Lerp -57.889229 -177.939266 _newtrack_0) 202.361636 129.0) false false)
          (Transformation|SetRelativeLocation (Variables|Default|GetDoor2) (Math|Vector|MakeVector (Math|Float|Lerp 59.0 174.0 _newtrack_0) 202.361636 129.0) false false))))))

(event EventActivate
  (params (Shooter%20Character%20Ref :type BP%20Shooter%20Character%20Object%20Reference))
  (if (not (Variables|Default|GetOpen%20Stste))
    (Default|ShowMessageInfoWIthAnim (Variables|/Game/_Game/Character/BP_ShooterCharacter.BP_ShooterCharacter_C|GetWBP_MainWidget%20ref Shooter%20Character%20Ref) "/Game/UI_Assert/T_U_Message_ContainerGreen.T_U_Message_ContainerGreen" "Interaction Success" "(R=1.000000,G=1.000000,B=1.000000,A=1.000000)")
    (Utilities|FlowControl|DoOnce false
      (:Completed
        (Audio|PlaySound2D "/Engine/VREditor/Sounds/UI/Enter_Simulate.Enter_Simulate" 1.5 1.0 0.0 0 0)
        (Variables|Default|SetOpen%20Stste true)
        (bind _newtrack_0 (Timeline|Timeline PlayFromStart)
          (:Update
            (Transformation|SetRelativeLocation (Variables|Default|GetDoor1) (Math|Vector|MakeVector (Math|Float|Lerp -57.889229 -177.939266 _newtrack_0) 202.361636 129.0) false false)
            (Transformation|SetRelativeLocation (Variables|Default|GetDoor2) (Math|Vector|MakeVector (Math|Float|Lerp 59.0 174.0 _newtrack_0) 202.361636 129.0) false false)))))))

(fn ConstructionScript)