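; Pressure-activated button that switches a referenced platform on while something is standing or resting on it.
; Box overlap events filter actors by Player, GrabbingObject or LaserBox tags, calling Activate on begin overlap and Deactivate on end overlap of the linked platform, each with a 2D sound.
; Overlaps are not counted, so any qualifying actor leaving deactivates the platform even if another remains.
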(event OnComponentBeginOverlap(Box)
  (params (OverlappedComponent :type Primitive%20Component%20Object%20Reference) (OtherActor :type Actor%20Object%20Reference) (OtherComp :type Primitive%20Component%20Object%20Reference) (OtherBodyIndex :type Integer) (bFromSweep :type Boolean) (SweepResult :type Hit%20Result%20Structure%20%28by%20ref%29))
  (if (Math|Boolean|ORBoolean (Actor|ActorHasTag OtherActor "Player") (Actor|ActorHasTag OtherActor "GrabbingObject") (Actor|ActorHasTag OtherActor "LaserBox"))
    (Default|Activate (Variables|Default|GetBP%20Platform%20ref))
    (Audio|PlaySound2D "/Engine/VREditor/Sounds/UI/Drop_Item_From_ContentBrowser.Drop_Item_From_ContentBrowser" 1.0 1.0 0.0 0 0)))

(event OnComponentEndOverlap(Box)
  (params (OverlappedComponent :type Primitive%20Component%20Object%20Reference) (OtherActor :type Actor%20Object%20Reference) (OtherComp :type Primitive%20Component%20Object%20Reference) (OtherBodyIndex :type Integer))
  (if (Math|Boolean|ORBoolean (Actor|ActorHasTag OtherActor "Player") (Actor|ActorHasTag OtherActor "GrabbingObject") (Actor|ActorHasTag OtherActor "LaserBox"))
    (Default|Deactivate (Variables|Default|GetBP%20Platform%20ref))
    (Audio|PlaySound2D "/Engine/VREditor/Sounds/UI/Dockable_Window_Close.Dockable_Window_Close" 1.0 1.0 0.0 0 0)))

(fn ConstructionScript)