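; BP_TimeDialation is a box trigger that applies a time dilation effect to the player while inside it.
; On overlap begin, it checks for BPI_Player, passes TimeDialationValue through an activate message, and shows an animated banner on the player's main widget.
; On overlap end, it sends the deactivate message through the same interface.
; A random left/right montage branch for the player is left disconnected and never runs.
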(event OnComponentBeginOverlap(Box)
  (params (OverlappedComponent :type Primitive%20Component%20Object%20Reference) (OtherActor :type Actor%20Object%20Reference) (OtherComp :type Primitive%20Component%20Object%20Reference) (OtherBodyIndex :type Integer) (bFromSweep :type Boolean) (SweepResult :type Hit%20Result%20Structure%20%28by%20ref%29))
  (if (Utilities|DoesObjectImplementInterface OtherActor "/Game/Blueprint/Interfaces-Enums/BPI_Player.BPI_Player_C")
    (Class|BPIPlayer|ActivateTimeDialation(Message) OtherActor (Variables|Default|GetTime%20Dialation%20Value))
    (bind _player_ref (Class|BPIPlayer|GetPlayerRef(Message) OtherActor))
    (Default|ShowMessageInfoWIthAnim (Variables|/Game/_Game/Character/BP_ShooterCharacter.BP_ShooterCharacter_C|GetWBP_MainWidget%20ref _player_ref) "/Game/UI_Assert/T_U_Message_ContainerPurple.T_U_Message_ContainerPurple" "SIIIUUU!" "(R=1.000000,G=1.000000,B=1.000000,A=1.000000)")))

(event OnComponentEndOverlap(Box)
  (params (OverlappedComponent :type Primitive%20Component%20Object%20Reference) (OtherActor :type Actor%20Object%20Reference) (OtherComp :type Primitive%20Component%20Object%20Reference) (OtherBodyIndex :type Integer))
  (if (Utilities|DoesObjectImplementInterface OtherActor "/Game/Blueprint/Interfaces-Enums/BPI_Player.BPI_Player_C")
    (Class|BPIPlayer|DeactivateTimeDialation(Message) OtherActor)
    (bind _player_ref (Class|BPIPlayer|GetPlayerRef(Message) OtherActor))))

(event EventBeginPlay)

(event Collision|EventActorBeginOverlap
  (params (OtherActor :type Actor%20Object%20Reference)))

(event EventTick
  (params (DeltaSeconds :type Float%20%28single-precision%29)))

(fn ConstructionScript)