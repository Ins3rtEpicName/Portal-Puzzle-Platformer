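; BP_Door is a two-stage puzzle door that consumes turrets to open.
; OpenDoor runs once, swinging one mesh via timeline, then revealing a Niagara effect and counter widget, starting a spinning mesh and arming a sphere trigger.
; Turret-tagged actors entering the sphere are released from the player's hold and destroyed with a blast, updating the widget count.
; At three turrets, a second timeline slides another mesh aside.
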(event OnComponentBeginOverlap(Sphere1)
  (params (OverlappedComponent :type Primitive%20Component%20Object%20Reference) (OtherActor :type Actor%20Object%20Reference) (OtherComp :type Primitive%20Component%20Object%20Reference) (OtherBodyIndex :type Integer) (bFromSweep :type Boolean) (SweepResult :type Hit%20Result%20Structure%20%28by%20ref%29))
  (if (Variables|Default|GetStartSphereTrace)
    (if (Actor|ActorHasTag OtherActor "Turret")
      (bind _asbp_shooter_character (Utilities|Casting|CastToBP_ShooterCharacter (Game|Player|GetPlayerPawn 0)))
      (Class|ShooterCharacter|ReleaseorDropObject _asbp_shooter_character)
      (Utilities|FlowControl|Delay 0.2)
      (Actor|DestroyActor OtherActor)
      (Effects|SpawnEmitteratLocation "/Game/Blast_VFX/FX/Blast.Blast" (Transformation|GetWorldLocation (Variables|Default|GetSphere1)))
      (Audio|PlaySound2D "/Game/_Game/Asserts/Sounds/Ambient/Explosion01.Explosion01" 1.0 1.0 0.0 0 0)
      (Math|Integer|IncrementInt (Variables|Default|GetTurretDestCount)
        (:%20%20
          (Default|SetCount (Variables|Default|GetWBP_ExplodeTurret%20Ref) (Variables|Default|GetTurretDestCount))
          (if (>= (Variables|Default|GetTurretDestCount) 3)
            (bind _newtrack_0 (Timeline|Timeline PlayFromStart)
              (:Update
                (Transformation|SetRelativeLocation (Variables|Default|GetStaticMesh1) (Math|Vector|MakeVector (Math|Float|Lerp 10.718661 -132.956284 _newtrack_0) 0.0 111.119157) false false))
              (:Finished
                (Audio|PlaySound2D "/Engine/VREditor/Sounds/UI/Enter_Simulate.Enter_Simulate" 1.5 1.0 0.0 0 0)))))))))

(event EventOpenDoor
  (Utilities|FlowControl|DoOnce false
    (:Completed
      (Variables|Default|SetRotationSpeed 1.5e+03)
      (Audio|PlaySound2D "/Engine/VREditor/Sounds/UI/Enter_Simulate.Enter_Simulate" 1.5 1.0 0.0 0 0)
      (bind _newtrack_0 (Timeline|Timeline_0 PlayFromStart)
        (:Update
          (Transformation|SetRelativeRotation (Variables|Default|GetStaticMesh5) (Math|Rotator|MakeRotator 0.0 0.0 (* _newtrack_0 9e+01)) false false))
        (:Finished
          (Rendering|SetVisibility (Variables|Default|GetNiagara) true false)
          (Variables|Default|SetStartSphereTrace true))))))

(event Collision|EventActorBeginOverlap
  (params (OtherActor :type Actor%20Object%20Reference)))

(event EventTick
  (params (DeltaSeconds :type Float%20%28single-precision%29))
  (if (Variables|Default|GetStartSphereTrace)
    (Transformation|AddLocalRotation (Variables|Default|GetStaticMesh4) (Math|Rotator|MakeRotator 0.0 0.0 (* DeltaSeconds (Variables|Default|GetRotationSpeed))) false false)))

(event EventBeginPlay
  (bind _aswbp_explode_turrets (Utilities|Casting|CastToWBP_ExplodeTurrets (UserInterface|GetWidget (Variables|Default|GetWidget))))
  (bind _output_get (Variables|Default|SetWBP_ExplodeTurret%20Ref _aswbp_explode_turrets))
  (Default|SetCount _output_get (Variables|Default|GetTurretDestCount))
  (Rendering|SetVisibility (Variables|Default|GetNiagara) false false))

(fn ConstructionScript)