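; Turret actor that swivels its ItemMesh2 along one axis chosen by LaserMode and toggles a widget's visibility.
; Tick plays one of four timelines, selected by LaserMode and Flipped, whose track scaled by RotateValue sets relative yaw for Left Right or pitch for Up Down.
; The widget is hidden on BeginPlay and shown or hidden through the ShowHideUIinBP event.
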(event EventBeginPlay
  (Rendering|SetVisibility (Variables|Default|GetWidget) false false))

(event EventTick
  (params (DeltaSeconds :type Float%20%28single-precision%29))
  (switch Utilities|FlowControl|Switch|SwitchonE_LaserMode (Variables|Settings|GetLaserMode)
    (:NewEnumerator1
      (if (Variables|Settings|GetFlipped)
        (bind _newtrack_0 (Timeline|Rotate Play)
          (:Update
            (Transformation|SetRelativeRotation (Variables|Default|GetItemMesh2) (Math|Rotator|MakeRotator 0.0 0.0 (* _newtrack_0 (Variables|Settings|GetRotate%20Value))) false false)))
        (else
          (bind _newtrack_0_2 (Timeline|RotateFlip Play)
            (:Update
              (Transformation|SetRelativeRotation (Variables|Default|GetItemMesh2) (Math|Rotator|MakeRotator 0.0 0.0 (* _newtrack_0_2 (Variables|Settings|GetRotate%20Value))) false false))))))
    (:NewEnumerator2
      (if (Variables|Settings|GetFlipped)
        (bind _newtrack_0_3 (Timeline|Timeline Play)
          (:Update
            (Transformation|SetRelativeRotation (Variables|Default|GetItemMesh2) (Math|Rotator|MakeRotator 0.0 (* _newtrack_0_3 (Variables|Settings|GetRotate%20Value)) 0.0) false false)))
        (else
          (bind _newtrack_0_4 (Timeline|Timeline_0 Play)
            (:Update
              (Transformation|SetRelativeRotation (Variables|Default|GetItemMesh2) (Math|Rotator|MakeRotator 0.0 (* _newtrack_0_4 (Variables|Settings|GetRotate%20Value)) 0.0) false false))))))))

(event EventShowHideUIinBP
  (params (Show :type Boolean))
  (Rendering|SetVisibility (Variables|Default|GetWidget) Show false))

(fn ConstructionScript)