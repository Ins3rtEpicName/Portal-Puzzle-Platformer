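; BP_BlowerSwitch is a toggleable lever switch that turns a linked wind blower, platform, launchpad or lab door on and off.
; Overlapping its box shows players an activate/deactivate prompt via BPI_Player.
; Activate plays a message, player montage, lever animation and sound, with a short delay lock blocking repeat use.
; ActivateType then dispatches to the device chosen by type, though timed lab doors only ever receive Activate.
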(event OnComponentBeginOverlap(Box)
  (params (OverlappedComponent :type Primitive%20Component%20Object%20Reference) (OtherActor :type Actor%20Object%20Reference) (OtherComp :type Primitive%20Component%20Object%20Reference) (OtherBodyIndex :type Integer) (bFromSweep :type Boolean) (SweepResult :type Hit%20Result%20Structure%20%28by%20ref%29))
  (if (Utilities|DoesObjectImplementInterface OtherActor "/Game/Blueprint/Interfaces-Enums/BPI_Player.BPI_Player_C")
    (if (Variables|Default|GetActivated)
      (Class|BPIPlayer|InteractButtonUIDisplay(Message) OtherActor "Press E to Deactivate")
      (else
        (Class|BPIPlayer|InteractButtonUIDisplay(Message) OtherActor "Press E to Activate")))))

(event Custom|ActivateType
  (params (BPType :type E_ActivateBPType%20Enum :default "NewEnumerator0") (Activate :type Boolean))
  (bind _bp_wind_blower_ref (Variables|References|GetBP%20Wind%20Blower%20Ref))
  (bind _bp_platform_ref (Variables|References|GetBP%20Platform%20ref))
  (bind _bp_launchpad_ref (Variables|References|GetBP%20Launchpad%20Ref))
  (bind _bp_labdoor_ref (Variables|References|GetBP%20LabDoor%20Ref))
  (switch Utilities|FlowControl|Switch|SwitchonE_ActivateBPType BPType
    (:NewEnumerator0
      (if Activate
        (Default|Activate _bp_wind_blower_ref)
        (else
          (Default|Deactivate _bp_wind_blower_ref))))
    (:NewEnumerator1
      (if Activate
        (Default|Activate _bp_platform_ref)
        (else
          (Default|Deactivate _bp_platform_ref))))
    (:NewEnumerator3
      (if Activate
        (Default|Activateee _bp_launchpad_ref)
        (else
          (Default|Deactivatee _bp_launchpad_ref))))
    (:NewEnumerator2
      (if Activate
        (Default|Activate _bp_labdoor_ref)
        (else
          (Default|Deactivate _bp_labdoor_ref))))
    (:NewEnumerator6
      (if true
        (Default|Activate (Variables|References|GetBP%20Timed%20LabDoor%20Ref))))))

(event EventActivate
  (params (Shooter%20Character%20Ref :type BP%20Shooter%20Character%20Object%20Reference))
  (bind _activatebptype (Variables|Default|GetActivateBPType))
  (bind _lever_switch (Variables|Default|GetLever_Switch))
  (if (not (Variables|Default|GetIn%20Progress))
    (if (not (Variables|Default|GetActivated))
      (Default|ShowMessageInfoWIthAnim (Variables|/Game/_Game/Character/BP_ShooterCharacter.BP_ShooterCharacter_C|GetWBP_MainWidget%20ref Shooter%20Character%20Ref) "/Game/UI_Assert/T_U_Message_ContainerPurple.T_U_Message_ContainerPurple" (Variables|Default|GetFlipMessagePrompt) "(R=1.000000,G=1.000000,B=1.000000,A=1.000000)")
      (Default|PlayMontage Shooter%20Character%20Ref "/Game/Blueprint/Animations/Emotes/Cosmic_Rift1_Montage.Cosmic_Rift1_Montage" 1.5)
      (Components|Animation|PlayAnimation _lever_switch "/Game/Blueprint/Wind_blower/Switch/Lever_Switch_Anim_Montage.Lever_Switch_Anim_Montage" false)
      (Variables|Default|SetActivated true)
      (Variables|Default|SetIn%20Progress true)
      (Audio|PlaySound2D "/Game/UI_Assert/Switch_On_Sound.Switch_On_Sound" 2.0 1.0 0.0 0 0)
      (Utilities|FlowControl|Delay 0.9)
      (Variables|Default|SetIn%20Progress false)
      (CallFunction|ActivateType _activatebptype true)
      (else
        (Default|ShowMessageInfoWIthAnim (Variables|/Game/_Game/Character/BP_ShooterCharacter.BP_ShooterCharacter_C|GetWBP_MainWidget%20ref Shooter%20Character%20Ref) "/Game/UI_Assert/T_U_Message_ContainerPurple.T_U_Message_ContainerPurple" (Variables|Default|GetFlopMessagePrompt) "(R=1.000000,G=1.000000,B=1.000000,A=1.000000)")
        (Default|PlayMontage Shooter%20Character%20Ref "/Game/Blueprint/Animations/Emotes/Cosmic_Rift1_Montage.Cosmic_Rift1_Montage" 1.5)
        (Components|Animation|PlayAnimation _lever_switch "/Game/Blueprint/Wind_blower/Switch/Off_Anim.Off_Anim" false)
        (Variables|Default|SetActivated false)
        (Variables|Default|SetIn%20Progress true)
        (Audio|PlaySound2D "/Game/UI_Assert/Switch_Off_sound.Switch_Off_sound" 2.0 1.0 0.0 0 0)
        (Utilities|FlowControl|Delay 0.9)
        (Variables|Default|SetIn%20Progress false)
        (CallFunction|ActivateType _activatebptype false)))))

(fn ConstructionScript)