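; BP_Launchpad is an interactable launchpad that throws the player along its Arrow's forward vector, scaled by LaunchForce.
; Overlapping players get an interact prompt; in one OperationType it always works, otherwise only while externally enabled through Can.
; Activate plays a timeline tilting the pad and raising the cylinder, then jumps, launches and rotates the character with a HUD message.
; A construction-script label shows the force, hidden on BeginPlay.
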(event OnComponentBeginOverlap(Box)
  (params (OverlappedComponent :type Primitive%20Component%20Object%20Reference) (OtherActor :type Actor%20Object%20Reference) (OtherComp :type Primitive%20Component%20Object%20Reference) (OtherBodyIndex :type Integer) (bFromSweep :type Boolean) (SweepResult :type Hit%20Result%20Structure%20%28by%20ref%29))
  (if (Utilities|DoesObjectImplementInterface OtherActor "/Game/Blueprint/Interfaces-Enums/BPI_Player.BPI_Player_C")
    (if (Utilities|Enum|Equal(Enum) (Variables|Default|GetOperationType) "NewEnumerator0")
      (Class|BPIPlayer|InteractButtonUIDisplay(Message) OtherActor "Interact with E" :!label _label)
      (elif (Variables|Default|GetCan?)
        (goto _label)))))

(event Custom|Activateee
  (Variables|Default|SetCan? true))

(event Custom|Deactivatee
  (Variables|Default|SetCan? false))

(event EventBeginPlay
  (Rendering|SetVisibility (Variables|Default|GetTextRender) false false))

(event EventActivate
  (params (Shooter%20Character%20Ref :type BP%20Shooter%20Character%20Object%20Reference))
  (bind _sm_launchpad (Variables|Default|GetSM_LaunchPad))
  (bind _cylinder (Variables|Default|GetCylinder))
  (bind _relativerotation (Variables|/Script/Engine.SceneComponent|GetRelativeRotation _cylinder))
  (bind _relativerotation_2 (Variables|/Script/Engine.SceneComponent|GetRelativeRotation _sm_launchpad))
  (if (Utilities|Enum|Equal(Enum) (Variables|Default|GetOperationType) "NewEnumerator0")
    (bind _launch (Timeline|Jumpad%20Timeline PlayFromStart)
      (:Update
        (Transformation|SetRelativeRotation _sm_launchpad (Math|Rotator|MakeRotator (Math|Float|Lerp 0.0 6e+01 _launch) (.pitch _relativerotation_2) (.yaw _relativerotation_2)) false false)
        (Transformation|SetRelativeLocation _cylinder (Math|Vector|MakeVector (.roll _relativerotation) (.pitch _relativerotation) (Math|Float|Lerp -3e+01 3e+01 _launch)) false false))
      (:Finished
        (Utilities|FlowControl|DoOnce false :!label _label
          (:Completed
            (Character|Jump Shooter%20Character%20Ref)
            (Character|LaunchCharacter Shooter%20Character%20Ref (* (Math|Vector|GetForwardVector (Variables|Default|GetArrow)) (Variables|Default|GetLaunch%20Force)) false false)
            (Default|ShowMessageInfoWIthAnim (Variables|/Game/_Game/Character/BP_ShooterCharacter.BP_ShooterCharacter_C|GetWBP_MainWidget%20ref Shooter%20Character%20Ref) "/Game/UI_Assert/T_U_Message_ContainerPurple.T_U_Message_ContainerPurple" "SIIIUUU!" "(R=1.000000,G=1.000000,B=1.000000,A=1.000000)")
            (Transformation|SetActorRotation Shooter%20Character%20Ref (Math|Conversions|RotationFromXVector (Math|Vector|GetForwardVector (Variables|Default|GetArrow))))
            (Utilities|FlowControl|Delay 0.2)
            (goto _label Reset)))))
    (elif (Variables|Default|GetCan?)
      (Timeline|Jumpad%20Timeline PlayFromStart))))

(fn ConstructionScript
  (Rendering|Components|TextRender|SetText (Variables|Default|GetTextRender) (Utilities|Text|ToText(String) (Utilities|String|Append "Launch Force : " (Utilities|String|ToString(Float) (Variables|Default|GetLaunch%20Force))))))