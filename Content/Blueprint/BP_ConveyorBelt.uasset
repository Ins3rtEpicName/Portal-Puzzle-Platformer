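; Conveyor belt actor that carries any actor overlapping its Box along the belt's facing direction.
; Each Tick it offsets every overlapping actor by the ConveyerSM forward vector scaled by Speed and delta time, without sweep or physics.
; The construction script gives the mesh a dynamic M_Conveyor material driven by Color, ArrowScale and ArrowSpeed, so the arrow visuals are set independently of the movement Speed.
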(event EventTick
  (params (DeltaSeconds :type Float%20%28single-precision%29))
  (for _array_element (Collision|GetOverlappingActors (Variables|Default|GetBox) 0 :!class /Script/Engine.PrimitiveComponent)
    (Transformation|AddActorWorldOffset _array_element (* (Math|Vector|GetForwardVector (Transformation|GetWorldRotation (Variables|Default|GetConveyer_SM))) (* DeltaSeconds (Variables|Default|GetSpeed))))))

(fn ConstructionScript
  (bind _conveyer_sm (Variables|Default|GetConveyer_SM))
  (bind _returnvalue (Rendering|Material|CreateDynamicMaterialInstance _conveyer_sm 0 "/Game/Blueprint/Conveyor-Belt/M_Conveyor.M_Conveyor" "None" :!class /Script/Engine.PrimitiveComponent))
  (Rendering|Material|SetMaterial _conveyer_sm 0 _returnvalue)
  (Rendering|Material|SetVectorParameterValue _returnvalue "Color" (Variables|Default|GetColor) :!class /Script/Engine.MaterialInstanceDynamic)
  (Rendering|Material|SetScalarParameterValue _returnvalue "X Scale" (Variables|Default|GetArrow%20Scale) :!class /Script/Engine.MaterialInstanceDynamic)
  (Rendering|Material|SetScalarParameterValue _returnvalue "X Speed" (Variables|Default|GetArrow%20Speed) :!class /Script/Engine.MaterialInstanceDynamic))