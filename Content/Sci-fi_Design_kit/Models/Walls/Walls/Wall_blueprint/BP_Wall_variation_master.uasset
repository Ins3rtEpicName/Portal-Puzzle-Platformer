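; Modular sci-fi wall Blueprint that assembles a wall from interchangeable base and top meshes.
; The Construction Script converts the BaseVariation and TopVariation selections to integers, indexes the matching mesh arrays, and assigns the results to the WallBase and WallTop static mesh components.
; The event graph holds only disabled placeholder events, so all logic runs at construction.
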(event EventBeginPlay)

(event Collision|EventActorBeginOverlap
  (params (OtherActor :type Actor%20Object%20Reference)))

(event EventTick
  (params (DeltaSeconds :type Float%20%28single-precision%29)))

(fn ConstructionScript
  (Utilities|FlowControl|Sequence
    (:then_0
      (Components|StaticMesh|SetStaticMesh (Variables|Default|GetWall_base) (Utilities|Array|Get(acopy) (LocalVariables|GetWall_base_variation) (Math|Conversions|ToInteger(Byte) (Variables|Default|GetBase_variation)))))
    (:then_1
      (Components|StaticMesh|SetStaticMesh (Variables|Default|GetWall_top) (Utilities|Array|Get(acopy) (LocalVariables|GetWall_top_variations) (Math|Conversions|ToInteger(Byte) (Variables|Default|GetTop_variation)))))))