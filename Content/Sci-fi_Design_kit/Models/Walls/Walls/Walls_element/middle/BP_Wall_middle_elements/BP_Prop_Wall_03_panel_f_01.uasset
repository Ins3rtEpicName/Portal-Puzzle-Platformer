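; Sci-fi wall panel prop Blueprint that animates eight fan components.
; Every Tick, all eight fans receive a local pitch rotation of RotationSpeed scaled by DeltaSeconds, so they spin at a frame-rate independent rate.
; The construction script is empty.
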(event EventTick
  (params (DeltaSeconds :type Float%20%28single-precision%29))
  (Transformation|AddLocalRotation (Variables|Default|GetFan_01) (* (Math|Rotator|MakeRotator 0.0 (Variables|Default|GetRotation_speed) 0.0) DeltaSeconds) false false))

(fn ConstructionScript)