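; Animated sci-fi big door prop that opens when something overlaps Door_collider and closes when the overlap ends.
; Separate open and close timelines lerp the left, right, top and bottom panels between stored positions and rotate the top and bottom center pieces.
; Both timelines play from start on every overlap event, with no actor filter.
; Open and close sounds play at world origin rather than at the door.
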(event OnComponentBeginOverlap(Door_collider)
  (params (OverlappedComponent :type Primitive%20Component%20Object%20Reference) (OtherActor :type Actor%20Object%20Reference) (OtherComp :type Primitive%20Component%20Object%20Reference) (OtherBodyIndex :type Integer) (bFromSweep :type Boolean) (SweepResult :type Hit%20Result%20Structure%20%28by%20ref%29))
  (Audio|PlaySoundatLocation "/Game/Sci-fi_Design_kit/Sounds/Wavs/Big_door_open.Big_door_open" "0, 0, 0" "0, 0, 0" 1.0 1.0 0.0 0 0 0 0)
  (bind (_direction _left_right _botton _top _rotation_open) (Timeline|Timeline_0 PlayFromStart)
    (:Update
      (Utilities|FlowControl|Sequence
        (:then_0
          (Transformation|SetRelativeLocation (Variables|Default|GetDoor_left) (Math|Vector|Lerp(Vector) (Variables|Default|GetLeft_first_position) (Variables|Default|GetLeft_second_position) _left_right) false false))
        (:then_1
          (Transformation|SetRelativeLocation (Variables|Default|GetDoor_right) (Math|Vector|Lerp(Vector) (Variables|Default|GetRight_first_position) (Variables|Default|GetRight_second_position) _left_right) false false))
        (:then_2
          (Transformation|SetRelativeLocation (Variables|Default|GetDoor_botton) (Math|Vector|Lerp(Vector) (Variables|Default|GetBotton_first_position) (Variables|Default|GetBotton_second_position) _botton) false false))
        (:then_3
          (Transformation|SetRelativeLocation (Variables|Default|GetDoor_top) (Math|Vector|Lerp(Vector) (Variables|Default|GetTop_first_position) (Variables|Default|GetTop_second_position) _top) false false))
        (:then_4
          (Transformation|SetRelativeRotation (Variables|Default|GetDoor_top_center) (Math|Rotator|Lerp(Rotator) (Variables|Default|GetTop_center_start) (Variables|Default|GetTop_center_end) _rotation_open) false false))
        (:then_5
          (Transformation|SetRelativeRotation (Variables|Default|GetDoor_botton_center) (Math|Rotator|Lerp(Rotator) (Variables|Default|GetBotton_center_start) (Variables|Default|GetBotton_center_end) _rotation_open) false false))))))

(event OnComponentEndOverlap(Door_collider)
  (params (OverlappedComponent :type Primitive%20Component%20Object%20Reference) (OtherActor :type Actor%20Object%20Reference) (OtherComp :type Primitive%20Component%20Object%20Reference) (OtherBodyIndex :type Integer))
  (Audio|PlaySoundatLocation "/Game/Sci-fi_Design_kit/Sounds/Wavs/Big_door_close.Big_door_close" "0, 0, 0" "0, 0, 0" 1.0 1.0 0.0 0 0 0 0)
  (bind (_direction _right_left_close _botton_top_closed _rotation_closed) (Timeline|Timeline_1 PlayFromStart)
    (:Update
      (Utilities|FlowControl|Sequence
        (:then_0
          (Transformation|SetRelativeLocation (Variables|Default|GetDoor_left) (Math|Vector|Lerp(Vector) (Variables|Default|GetLeft_second_position) (Variables|Default|GetLeft_first_position) _right_left_close) false false))
        (:then_1
          (Transformation|SetRelativeLocation (Variables|Default|GetDoor_right) (Math|Vector|Lerp(Vector) (Variables|Default|GetRight_second_position) (Variables|Default|GetRight_first_position) _right_left_close) false false))
        (:then_2
          (Transformation|SetRelativeLocation (Variables|Default|GetDoor_botton) (Math|Vector|Lerp(Vector) (Variables|Default|GetBotton_second_position) (Variables|Default|GetBotton_first_position) _botton_top_closed) false false))
        (:then_3
          (Transformation|SetRelativeLocation (Variables|Default|GetDoor_top) (Math|Vector|Lerp(Vector) (Variables|Default|GetTop_second_position) (Variables|Default|GetTop_first_position) _botton_top_closed) false false))
        (:then_6
          (Transformation|SetRelativeRotation (Variables|Default|GetDoor_top_center) (Math|Rotator|Lerp(Rotator) (Variables|Default|GetTop_center_end) (Variables|Default|GetTop_center_start) _rotation_closed) false false))
        (:then_7
          (Transformation|SetRelativeRotation (Variables|Default|GetDoor_botton_center) (Math|Rotator|Lerp(Rotator) (Variables|Default|GetBotton_center_end) (Variables|Default|GetBotton_center_start) _rotation_closed) false false))))))

(fn ConstructionScript)