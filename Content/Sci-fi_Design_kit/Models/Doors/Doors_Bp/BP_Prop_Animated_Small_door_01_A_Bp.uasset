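; Animated small sci-fi door prop that slides two panels open when something overlaps its trigger and closed when the overlap ends.
; The Vertical_door timeline drives each panel from its own track, lerping relative location between start and end points.
; Overlaps are unfiltered and restart the timeline from either extreme, so interrupted motion snaps.
; Open and close sounds play at world origin rather than at the door.
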(event OnComponentEndOverlap(Door_trigger)
  (params (OverlappedComponent :type Primitive%20Component%20Object%20Reference) (OtherActor :type Actor%20Object%20Reference) (OtherComp :type Primitive%20Component%20Object%20Reference) (OtherBodyIndex :type Integer))
  (Audio|PlaySoundatLocation "/Game/Sci-fi_Design_kit/Sounds/Wavs/Small_door_close.Small_door_close" "0, 0, 0" "0, 0, 0" 1.0 1.0 0.0 0 0 0 0)
  (bind (_direction _top _botton) (Timeline|Vertical_door ReverseFromEnd)
    (:Update
      (Utilities|FlowControl|Sequence
        (:then_0
          (Transformation|SetRelativeLocation (Variables|Default|GetSmall_door_Left) (Math|Vector|Lerp(Vector) (Variables|Default|GetLeft_Start) (Variables|Default|GetLeft_End) _botton) false false))
        (:then_1
          (Transformation|SetRelativeLocation (Variables|Default|GetSmall_door_Right) (Math|Vector|Lerp(Vector) (Variables|Default|GetRight_Start) (Variables|Default|GetRight_End) _top) false false))))))

(event OnComponentBeginOverlap(Door_trigger)
  (params (OverlappedComponent :type Primitive%20Component%20Object%20Reference) (OtherActor :type Actor%20Object%20Reference) (OtherComp :type Primitive%20Component%20Object%20Reference) (OtherBodyIndex :type Integer) (bFromSweep :type Boolean) (SweepResult :type Hit%20Result%20Structure%20%28by%20ref%29))
  (Audio|PlaySoundatLocation "/Game/Sci-fi_Design_kit/Sounds/Wavs/Small_door_open.Small_door_open" "0, 0, 0" "0, 0, 0" 1.0 1.0 0.0 0 0 0 0)
  (bind (_direction _top _botton) (Timeline|Vertical_door PlayFromStart)
    (:Update
      (Utilities|FlowControl|Sequence
        (:then_0
          (Transformation|SetRelativeLocation (Variables|Default|GetSmall_door_Left) (Math|Vector|Lerp(Vector) (Variables|Default|GetLeft_Start) (Variables|Default|GetLeft_End) _botton) false false))
        (:then_1
          (Transformation|SetRelativeLocation (Variables|Default|GetSmall_door_Right) (Math|Vector|Lerp(Vector) (Variables|Default|GetRight_Start) (Variables|Default|GetRight_End) _top) false false))))))

(fn ConstructionScript)