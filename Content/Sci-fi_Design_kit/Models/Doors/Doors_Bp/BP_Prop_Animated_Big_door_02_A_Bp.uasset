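; Animated vertical big door prop for a sci-fi kit that opens and closes automatically through a trigger volume.
; Beginning overlap plays the Vertical_door timeline from the start, lerping the top and bottom panels between their start and end relative locations on separate tracks.
; Ending overlap reverses the timeline from its end, with no filter on the overlapping actor.
; Open and close sounds play at the world origin rather than the door's location.
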(event OnComponentEndOverlap(Door_trigger)
  (params (OverlappedComponent :type Primitive%20Component%20Object%20Reference) (OtherActor :type Actor%20Object%20Reference) (OtherComp :type Primitive%20Component%20Object%20Reference) (OtherBodyIndex :type Integer))
  (Audio|PlaySoundatLocation "/Game/Sci-fi_Design_kit/Sounds/Wavs/Vertical_door_close.Vertical_door_close" "0, 0, 0" "0, 0, 0" 1.0 1.0 0.0 0 0 0 0)
  (bind (_direction _top _botton) (Timeline|Vertical_door ReverseFromEnd)
    (:Update
      (Utilities|FlowControl|Sequence
        (:then_0
          (Transformation|SetRelativeLocation (Variables|Default|Getvertical_door_botton) (Math|Vector|Lerp(Vector) (Variables|Default|GetDoor_botton_Start) (Variables|Default|GetDoor_botton_End) _botton) false false))
        (:then_1
          (Transformation|SetRelativeLocation (Variables|Default|Getvertical_door_top) (Math|Vector|Lerp(Vector) (Variables|Default|GetDoor_top_Start) (Variables|Default|GetDoor_top_End) _top) false false))))))

(event OnComponentBeginOverlap(Door_trigger)
  (params (OverlappedComponent :type Primitive%20Component%20Object%20Reference) (OtherActor :type Actor%20Object%20Reference) (OtherComp :type Primitive%20Component%20Object%20Reference) (OtherBodyIndex :type Integer) (bFromSweep :type Boolean) (SweepResult :type Hit%20Result%20Structure%20%28by%20ref%29))
  (Audio|PlaySoundatLocation "/Game/Sci-fi_Design_kit/Sounds/Wavs/Vertical_door_open.Vertical_door_open" "0, 0, 0" "0, 0, 0" 1.0 1.0 0.0 0 0 0 0)
  (bind (_direction _top _botton) (Timeline|Vertical_door PlayFromStart)
    (:Update
      (Utilities|FlowControl|Sequence
        (:then_0
          (Transformation|SetRelativeLocation (Variables|Default|Getvertical_door_botton) (Math|Vector|Lerp(Vector) (Variables|Default|GetDoor_botton_Start) (Variables|Default|GetDoor_botton_End) _botton) false false))
        (:then_1
          (Transformation|SetRelativeLocation (Variables|Default|Getvertical_door_top) (Math|Vector|Lerp(Vector) (Variables|Default|GetDoor_top_Start) (Variables|Default|GetDoor_top_End) _top) false false))))))

(fn ConstructionScript)