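; Spline-based wire prop for the science lab, built in the construction script as a chain of spline mesh components.
; SplineMeshVar selects segments between spline points or at fixed Spacing along the spline length, with tangents scaled by TangentScale.
; WireVar picks one of six component variants, the last three using two material slots, and WireSize scales each segment.
; Per-segment dynamic instances of MI_Wire receive colours, specular, roughness and a TextureVar-selected texture set.
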(fn ConstructionScript
  (|Wire))